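; BP_Boo is a ghost enemy, styled after Boo, that stalks the player only while out of view.
; Each tick it faces the player and uses ProjectWorldToScreen success as its visibility test, ignoring occlusion.
; When seen it halts and fades via a dynamic material's Opacity; otherwise it turns opaque and advances along its mesh's right vector without sweeping.
; Overlapping BP_Character triggers GameOver, then loads EntryLevel after a delay.
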(event `self.ReceiveBeginPlay`
  (bind _returnvalue (`PrimitiveComponent.CreateDynamicMaterialInstance` (`self.Boo`) 0 "/Game/MAterials/Boo_Mat.Boo_Mat" "None"))
  (set `self.MaterialReference` _returnvalue))

(event `/Game/Blueprints/BP_Interactive_Interface.Interact`)

(event `self.ReceiveTick`
  (params (DeltaSeconds :type "Float (single-precision)"))
  (bind _materialreference (`self.MaterialReference`))
  (`self.LookAtPlayer`)
  (bind _output_get (set `self.IsVisible` (`.ReturnValue` (`GameplayStatics.ProjectWorldToScreen` (`GameplayStatics.GetPlayerController` 0) (`self.K2_GetActorLocation`)))))
  (if _output_get
    (bind _output_get_2 (set `self.CurrentTransparency` (`KismetMathLibrary.FMax` (- (`self.CurrentTransparency`) (* (`self.TransparencyPerSecond`) (`GameplayStatics.GetWorldDeltaSeconds`))) 0.15)))
    (`MaterialInstanceDynamic.SetScalarParameterValue` _materialreference "Opacity" _output_get_2)
    (else
      (`self.MoveToPlayer`)
      (`MaterialInstanceDynamic.SetScalarParameterValue` _materialreference "Opacity" 1.0)
      (set `self.CurrentTransparency` 1.0)))
  (`PrimitiveComponent.SetMaterial` (`self.Boo`) 0 _materialreference))

(event `self.Boo.OnComponentBeginOverlap`
  (params (OverlappedComponent :type "PrimitiveComponent Object Reference") (OtherActor :type "Actor Object Reference") (OtherComp :type "PrimitiveComponent Object Reference") (OtherBodyIndex :type Integer) (bFromSweep :type Boolean) (SweepResult :type "HitResult Structure (by ref)"))
  (bind _asbp_character (cast `/Game/Blueprints/BP_Character` OtherActor))
  (`/Game/Blueprints/BP_Character.GameOver` _asbp_character)
  (set `/Game/Blueprints/BP_Character.IsCaught` true _asbp_character)
  (`SceneComponent.SetVisibility` (`self.Boo`) true false)
  (`KismetSystemLibrary.PrintString` "You were caught! Try to survive as long as you can!")
  (`KismetSystemLibrary.Delay` 5.0)
  (`GameplayStatics.OpenLevel` "EntryLevel"))

(fn `LookAtPlayer`
  (`self.K2_SetActorRotation` (`KismetMathLibrary.FindLookAtRotation` (`self.K2_GetActorLocation`) (`self.K2_GetActorLocation` (`GameplayStatics.GetPlayerCharacter` 0)))))

(fn `MoveToPlayer`
  (`self.K2_SetActorLocation` (+ (`self.K2_GetActorLocation`) (* (`SceneComponent.GetRightVector` (`self.Boo`)) (* (`self.MovementSpeed`) (`GameplayStatics.GetWorldDeltaSeconds`))))))

(fn `UserConstructionScript`
  (bind _returnvalue (`PrimitiveComponent.CreateDynamicMaterialInstance` (`self.Boo`) 0 "/Game/MAterials/Boo_Mat.Boo_Mat" "None"))
  (set `self.MaterialReference` _returnvalue))