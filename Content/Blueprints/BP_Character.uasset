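; Player character steered by gaze, walking along the camera's forward vector while touch is held, with mouse axes turning the view.
; Each tick a camera line trace stores any hit actor implementing BP_Interactive_Interface, so a touch interacts with it instead of starting movement.
; Being caught disables input, and hitting BP_Boo only prints a message.
; GameOver shows the game-over widget; teleport logic is left unconnected.
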(event `self.ReceiveBeginPlay`)

(event `self.ReceiveTick`
  (params (DeltaSeconds :type "Float (single-precision)"))
  ;[1 1 1] Movement
  (if (`self.IsCaught`)
    (`self.DisableInput` null)
    (else
      (`self.GazeCheck`)
      (`PawnMovementComponent.AddInputVector` (`self.CharacterMovement`) (* (`SceneComponent.GetForwardVector` (`self.Camera`)) (* (`self.MovementSpeed`) DeltaSeconds)) false))))

(event `InputAction|touch`
  (params (Key :type "Key Structure"))
  (bind _interactiveactor (`self.InteractiveActor`))
  ;[1 1 1] Input
  (:`Pressed`
    (`/Engine/EditorBlueprintResources/StandardMacros.IsValid` _interactiveactor
      (:`Is Valid`
        (message `/Game/Blueprints/BP_Interactive_Interface.Interact` _interactiveactor))
      (:`Is Not Valid`
        (set `self.MovementSpeed` 90.0))))
  (:`Released`
    (set `self.MovementSpeed` 0.0)))

(event `InputAxis|mouseX`
  (params (AxisValue :type "Float (single-precision)"))
  ;[1 1 1] Input
  (`self.AddControllerYawInput` AxisValue))

(event `InputAxis|mouseY`
  (params (AxisValue :type "Float (single-precision)"))
  ;[1 1 1] Input
  (`self.AddControllerPitchInput` AxisValue))

(event `GazeCheck`
  (bind _camera (`self.Camera`))
  (bind _returnvalue (`SceneComponent.K2_GetComponentLocation` _camera))
  ;[1 1 1] Gaze check
  (bind _outhit (`KismetSystemLibrary.LineTraceSingle` :`Start` _returnvalue :`End` (+ _returnvalue (* (`SceneComponent.GetForwardVector` _camera) 2000)) :`TraceChannel` "TraceTypeQuery1" :`DrawDebugType` "ForOneFrame"))
  (bind (_bblockinghit _binitialoverlap _time _distance _location _impactpoint _normal _impactnormal _physmat _hitactor) (`GameplayStatics.BreakHitResult` _outhit))
  (set `self.EyeContact` _location)
  (if (`KismetSystemLibrary.DoesImplementInterface` _hitactor "/Game/Blueprints/BP_Interactive_Interface.BP_Interactive_Interface_C")
    (set `self.InteractiveActor` _hitactor)
    (set `self.CanTeleport` false)
    (else
      (set `self.InteractiveActor` null)
      (set `self.CanTeleport` true))))

(event `self.CapsuleComponent.OnComponentHit`
  (params (HitComponent :type "PrimitiveComponent Object Reference") (OtherActor :type "Actor Object Reference") (OtherComp :type "PrimitiveComponent Object Reference") (NormalImpulse :type "Vector Structure") (Hit :type "HitResult Structure (by ref)"))
  (cast `/Game/Blueprints/BP_Boo` OtherActor)
  (`KismetSystemLibrary.PrintString` "BOO!"))

(fn `GameOver`
  (bind _returnvalue (`|CreateWidget` "/Game/Blueprints/BP_GameOver.BP_GameOver_C" (`GameplayStatics.GetPlayerController` 0)))
  (`UserWidget.AddToViewport` _returnvalue 0))

(fn `UserConstructionScript`)