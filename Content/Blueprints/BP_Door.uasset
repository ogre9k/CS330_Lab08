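; Interactable door actor that toggles open and closed when its Interact event fires.
; Interact calls RotateDoor, which checks IsOpen, snaps the Door component between two fixed rotations, flips the flag and prints the new state.
; The rotation is instant and set in world space, so it ignores the placed actor's orientation.
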(event `/Game/Blueprints/BP_Interactive_Interface.Interact`
  (`self.RotateDoor`))

(fn `RotateDoor`
  (bind _door (`self.Door`))
  (if (`self.IsOpen`)
    (`SceneComponent.K2_SetWorldRotation` :`self` _door)
    (set `self.IsOpen` false)
    (`KismetSystemLibrary.PrintString` "Door is Closed!")
    (else
      (`SceneComponent.K2_SetWorldRotation` _door (struct :`Yaw` -90.0) false false)
      (set `self.IsOpen` true)
      (`KismetSystemLibrary.PrintString` "Door is Open!"))))

(fn `UserConstructionScript`)